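; Market barrow pawn Blueprint that displays the resource it is transporting on a text label.
; On BeginPlay it caches the BPWidget_Text from its widget component and clears the text.
; Resource events set the label to the type and amount on pickup and clear it on reset.
; Each tick it billboards the widget against the player camera's forward vector, keeping it parallel to the view rather than pointed at the camera.
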(event `self.ReceiveBeginPlay`
  (bind _asbpwidget_text (cast `/Game/Blueprints/UI/Utility/BPWidget_Text` (`WidgetComponent.GetUserWidgetObject` (`self.Widget`))))
  (bind _output_get (set `self.UserWidget` _asbpwidget_text))
  (set `/Game/Blueprints/UI/Utility/BPWidget_Text.Text` "" _output_get))

(event `self.BPEvent_OnGetResource`
  (params (TransportedResource :type "Resource Structure (by ref)"))
  (set `/Game/Blueprints/UI/Utility/BPWidget_Text.Text` (`KismetTextLibrary.Conv_StringToText` (`KismetStringLibrary.Concat_StrStr` (`|GetEnumeratorNameAsString` TransportedResource_Type) ": " (`KismetStringLibrary.Conv_IntToString` TransportedResource_Amount))) (`self.UserWidget`)))

(event `self.BPEvent_OnReset`
  (set `/Game/Blueprints/UI/Utility/BPWidget_Text.Text` "  " (`self.UserWidget`)))

(event `self.ReceiveTick`
  (params (DeltaSeconds :type "Float (single-precision)"))
  (bind _playercameramanager (`PlayerController.PlayerCameraManager` (`UtilityFunctionLibrary.GetFirstEtosPlayerController`)))
  (bind _returnvalue (`PlayerCameraManager.GetCameraLocation` _playercameramanager))
  ;[1 1 1] Rotate Widget to camera
  (`/Engine/EditorBlueprintResources/StandardMacros.IsValid` _playercameramanager
    (:`Is Valid`
      (`SceneComponent.K2_SetWorldRotation` (`self.Widget`) (`KismetMathLibrary.FindLookAtRotation` (+ _returnvalue (`KismetMathLibrary.GetForwardVector` (`PlayerCameraManager.GetCameraRotation` _playercameramanager))) _returnvalue) false false))))

(fn `UserConstructionScript`)